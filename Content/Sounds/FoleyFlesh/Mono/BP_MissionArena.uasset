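; BP_MissionArena is an overlap volume that kills a marine who stays outside the mission area too long.
; Begin and end overlap with BP_Marine set its InsideMissionArena flag, and leaving starts a timeline from zero.
; Each timeline update stops playback if the marine is back inside, otherwise copies the elapsed time to LastMissionArenaTime.
; When the timeline finishes, it prints the time and calls Death on the marine.
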(event `self.ReceiveActorBeginOverlap`
  (params (OtherActor :type "Actor Object Reference"))
  (bind _asbp_marine (cast `/Game/Blueprints/BP_Marine` OtherActor))
  (bind _output_get (set `self.As BP Marine` _asbp_marine))
  (set `/Game/Blueprints/BP_Marine.InsideMissionArena` true _output_get))

(event `self.ReceiveActorEndOverlap`
  (params (OtherActor :type "Actor Object Reference"))
  (bind _asbp_marine (cast `/Game/Blueprints/BP_Marine` OtherActor))
  (bind _output_get (set `self.As BP Marine` _asbp_marine))
  (set `/Game/Blueprints/BP_Marine.InsideMissionArena` false _output_get)
  (bind (_direction _time) (`Timeline|Timeline` :!via `PlayFromStart` :!label _label)
    (:`Update`
      (if (`/Game/Blueprints/BP_Marine.InsideMissionArena` _output_get)
        (goto _label :!via `Stop`)
        (else
          (set `/Game/Blueprints/BP_Marine.lastMissionArenaTime` _time _output_get))))
    (:`Finished`
      (`KismetSystemLibrary.PrintString` (`KismetStringLibrary.Conv_DoubleToString` _time))
      (`/Game/Blueprints/BP_Marine.Death` _output_get))))

(fn `UserConstructionScript`)