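; BP_PickHealth is a health pickup that the player marine collects by touching it.
; On BeginPlay it rolls a random heal amount from zero up to a limit that scales with the wave count in GM_BaseGameMode.
; On overlap with a BP_Marine it passes that amount to HealthAdd, plays a pickup sound at its location and destroys itself.
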(event `self.ReceiveBeginPlay`
  (bind _asgm_base_game_mode (cast `/Game/Blueprints/GameMode/GM_BaseGameMode` (`GameplayStatics.GetGameMode`)))
  (set `self.Health` (`KismetMathLibrary.RandomFloatInRange` 0.0 (`KismetMathLibrary.Conv_IntToDouble` (* (`/Game/Blueprints/GameMode/GM_BaseGameMode.WaveCount` _asgm_base_game_mode) 50)))))

(event `self.ReceiveActorBeginOverlap`
  (params (OtherActor :type "Actor Object Reference"))
  (bind _asbp_marine (cast `/Game/Blueprints/BP_Marine` OtherActor))
  (`/Game/Blueprints/BP_Marine.HealthAdd` _asbp_marine (`self.Health`))
  (`GameplayStatics.SpawnSoundAtLocation` "/Game/Sounds/Stingers/Stereo/StingerPickup_Health01_Stereo.StingerPickup_Health01_Stereo" (`self.K2_GetActorLocation`) (struct) 1.0 1.0 0.0 null null)
  (`self.K2_DestroyActor`))

(fn `UserConstructionScript`)