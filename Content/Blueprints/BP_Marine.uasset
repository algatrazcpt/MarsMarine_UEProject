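; Player marine character with world-axis movement, a WBP_Ui HUD, kill count, pause toggle and a key to open the Mars level.
; Fire macros switch between single and automatic rifle effects, with a looping timer driving auto-fire line traces from the muzzle that apply damage.
; Incoming damage fades the camera and, at zero health, triggers death, stopping movement and fire.
; Bonus functions raise damage and heal, or raise max health when already full.
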(event `self.ReceiveAnyDamage`
  (params (Damage :type "Float (single-precision)") (DamageType :type "DamageType Object Reference") (InstigatedBy :type "Controller Object Reference") (DamageCauser :type "Actor Object Reference"))
  (if (`self.playerIsAlive`)
    (bind _isalive (`self.TakeDamage` Damage))
    (`PlayerCameraManager.StartCameraFade` :`self` (`GameplayStatics.GetPlayerCameraManager` 0) :`FromAlpha` 0.5 :`Duration` 1.0 :`bShouldFadeAudio` true)
    (bind _output_get (set `self.playerIsAlive` _isalive))
    (if (not _output_get)
      (`self.Death`))))

(event `self.ReceiveBeginPlay`
  (bind _returnvalue (`|CreateWidget` "/Game/UI/WBP_Ui.WBP_Ui_C" null self))
  (bind _output_get (set `self.CurrentUi` _returnvalue))
  (`UserWidget.AddToViewport` _output_get 0)
  (set `self.CurrentHealth` (`self.Health`)))

(event `InputAxis|Forward/Backward`
  (params (AxisValue :type "Float (single-precision)"))
  ; Move
  (`self.AddMovementInput` (1.0 0.0 0.0) AxisValue))

(event `InputAxis|Left/right`
  (params (AxisValue :type "Float (single-precision)"))
  ; Move
  (`self.AddMovementInput` (0.0 1.0 0.0) AxisValue))

(event `self.ReceiveTick`
  (params (DeltaSeconds :type "Float (single-precision)"))
  (`self.Aiming` 0.0))

(event `InputVectorAxis|Mouse2D`
  (params (AxisValue :type "Vector Structure")))

(event `InputAction|FireButton`
  (params (Key :type "Key Structure"))
  ; Fire
  (:`Pressed`
    (if (`self.playerIsAlive`)
      (`self.Fire`
        (:`then`
          (`self.Trace`)
          (if (`KismetSystemLibrary.K2_IsValidTimerHandle` (`self.Timer`))
            (`KismetSystemLibrary.K2_UnPauseTimer` null "Trace")
            (else
              (bind _returnvalue (`KismetSystemLibrary.K2_SetTimer` null "Trace" (/ 1.0 (`self.FireRate`)) true))
              (set `self.Timer` _returnvalue))))
        (:`then2`
          (`self.Trace`)))))
  (:`Released`
    (if (`self.playerIsAlive`)
      (`self.StopFire`)
      (`KismetSystemLibrary.K2_PauseTimer` null "Trace"))))

(event `InputAction|FireModeButton`
  (params (Key :type "Key Structure"))
  (:`Pressed`
    (set `self.FireModeAuto` (not (`self.FireModeAuto`)))))

(event `Key|T`
  (params (Key :type "Key Structure"))
  (:`Pressed`
    (`GameplayStatics.OpenLevel` "Mars")))

(event `Key|P` :paused true
  (params (Key :type "Key Structure"))
  (:`Pressed`
    (bind _isa (`/Engine/EditorBlueprintResources/StandardMacros.FlipFlop`)
      (:`A`
        _)
      (:`B`
        _))
    (`GameplayStatics.SetGamePaused` _isa)))

(fn `Aiming`
  (params (Value :type "Float (double-precision)"))
  ; Comment
  (if (`self.playerIsAlive`)
    (`self.AddControllerYawInput` (`KismetMathLibrary.FClamp` Value -2.0 2.0))))

(fn `DamageAdd`
  (params (Value :type "Float (double-precision)"))
  (set `self.Base Damage` (+ Value (`self.Base Damage`))))

(fn `Death`
  (`GameplayStatics.PlaySoundAtLocation` "/Game/Sounds/Stingers/Stereo/Stinger_PlayerDeath_Stereo_Cue.Stinger_PlayerDeath_Stereo_Cue" (`self.K2_GetActorLocation`) (struct) 1.0 1.0 0.0 null null null null)
  (set `self.playerIsAlive` false)
  (`ActorComponent.Deactivate` (`self.CharacterMovement`))
  (`PlayerCameraManager.StartCameraFade` :`self` (`GameplayStatics.GetPlayerCameraManager` 0) :`FromAlpha` 0.5 :`Duration` 2.0 :`bHoldWhenFinished` true)
  (`self.StopFire`)
  (`KismetSystemLibrary.K2_PauseTimer` null "Trace"))

(fn `HealthAdd`
  (params (Value :type "Float (double-precision)"))
  (if (== (`self.CurrentHealth`) (`self.Health`))
    ; BonusMaxHealthAdded
    (bind _output_get (set `self.Health` (+ Value (`self.Health`))))
    (set `self.CurrentHealth` _output_get)
    (else
      ; CurrentHealthAdded
      (set `self.CurrentHealth` (`KismetMathLibrary.FClamp` (+ Value (`self.CurrentHealth`)) 0.0 (`self.Health`)))
      (set `self.Health` (`self.Health`)))))

(fn `IsMouseDeadZone`
  (returns (IsAboveDeadZone :type Boolean))
  (return (> (`KismetMathLibrary.VSize2D` (`self.MouseVelocity`)) (`self.MouseDeadZone`))))

(fn `KillEnemy`
  (set `self.KillCount` (+ (`self.KillCount`) 1)))

(fn `MouseVelocity`
  (returns (Output_Get :type "Vector2D Structure"))
  (bind (_deltax _deltay) (`PlayerController.GetInputMouseDelta` (`GameplayStatics.GetPlayerController` 0)))
  (return (/ (`KismetMathLibrary.MakeVector2D` _deltax _deltay) (`GameplayStatics.GetWorldDeltaSeconds`))))

(fn `SpawnHitImpact`
  (params (Location :type "Vector Structure"))
  (`GameplayStatics.SpawnEmitterAtLocation` "/Game/Effects/Weapons/Impacts/P_AssaultRifle_IH.P_AssaultRifle_IH" Location))

(fn `StopFire`
  (bind _shootsound (`self.ShootSound`))
  (`/Engine/EditorBlueprintResources/StandardMacros.IsValid` _shootsound
    (:`Is Valid`
      (`AudioComponent.Stop` _shootsound))
    (:`Is Not Valid`
      _))
  (`ActorComponent.Deactivate` (`self.P_AssaultRifle_MF`))
  (`GameplayStatics.SpawnSoundAttached` "/Game/Sounds/Weapon_AssaultRifle/Stereo/RiffleEnd_cue.RiffleEnd_cue" (`self.Riffle`) "None" (0.0 0.0 0.0) (struct) "KeepRelativeOffset" false 1.0 1.0 0.0 null null))

(fn `TakeDamage`
  (params (Damage :type "Float (double-precision)"))
  (returns (IsAlive :type Boolean))
  (bind _output_get (set `self.CurrentHealth` (`KismetMathLibrary.FClamp` (- (`self.CurrentHealth`) Damage) 0.0 (`self.Health`))))
  (return (> _output_get 0.0)))

(fn `Trace`
  (bind _outhit (`KismetSystemLibrary.LineTraceSingle` (`self.TraceStartLocation`) (`self.TraceEndLocation`) "TraceTypeQuery1"))
  (bind (_bblockinghit _binitialoverlap _time _distance _location _impactpoint _normal _impactnormal _physmat _hitactor) (`GameplayStatics.BreakHitResult` _outhit))
  (if _bblockinghit
    (`self.SpawnHitImpact` _location)
    (`GameplayStatics.ApplyDamage` _hitactor (`self.Base Damage`))
    (return)))

(fn `TraceEndLocation`
  (returns (ReturnValue :type "Vector Structure"))
  (return (+ (`self.TraceStartLocation`) (* (`KismetMathLibrary.GetForwardVector` (`self.GetControlRotation`)) (`self.AttackRange`)))))

(fn `TraceStartLocation`
  (returns (ReturnValue :type "Vector Structure"))
  (return (`SceneComponent.GetSocketLocation` (`self.P_AssaultRifle_MF`) "MuzzleFlashSocket")))

(fn `UserConstructionScript`)