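; BP_RiffleBuff is a one-shot damage pickup for the marine.
; On BeginPlay it rolls a random bonus between zero and twice the game mode's current wave count, so potential strength scales with wave progression.
; When a BP_Marine overlaps it, it passes that bonus to DamageAdd, plays a 2D ammo pickup sound and destroys itself.
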(event `self.ReceiveBeginPlay`
  (bind _asgm_base_game_mode (cast `/Game/Blueprints/GameMode/GM_BaseGameMode` (`GameplayStatics.GetGameMode`)))
  (set `self.DamageUp` (`KismetMathLibrary.RandomFloatInRange` 0.0 (`KismetMathLibrary.Conv_IntToDouble` (* (`/Game/Blueprints/GameMode/GM_BaseGameMode.WaveCount` _asgm_base_game_mode) 2)))))

(event `self.ReceiveActorBeginOverlap`
  (params (OtherActor :type "Actor Object Reference"))
  (bind _asbp_marine (cast `/Game/Blueprints/BP_Marine` OtherActor))
  (`/Game/Blueprints/BP_Marine.DamageAdd` _asbp_marine (`self.DamageUp`))
  (`GameplayStatics.SpawnSound2D` "/Game/Sounds/Weapon_AssaultRifle/Stereo/Weapon_AssaultRifle_AmmoPickup01_Stereo.Weapon_AssaultRifle_AmmoPickup01_Stereo" 1.0 1.0 0.0 null)
  (`self.K2_DestroyActor`))

(fn `UserConstructionScript`)