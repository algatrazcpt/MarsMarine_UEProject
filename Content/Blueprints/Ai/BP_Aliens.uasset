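; Alien enemy that chases the Marine player and loops a melee attack montage while the player is in its AttackRadius.
; Spawned plays a teleport montage and randomly rolls health and damage buffs scaled by difficulty, swapping materials to show them.
; Tick re-issues AI MoveTo through a resettable DoOnce, and damage lowers clamped health.
; A Death macro credits the kill, rolls pickup drops and despawns through the game mode.
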(event `self.ReceiveBeginPlay`
  (bind _asgm_base_game_mode (cast `/Game/Blueprints/GameMode/GM_BaseGameMode` (`GameplayStatics.GetGameMode`)))
  (set `self.As GM Base Game Mode` _asgm_base_game_mode))

(event `Spawned`
  (params (Difficulty :type "Float (double-precision)"))
  (`self.ChangeMaterialSystemBuff` Difficulty)
  (bind _asbp_marine (cast `/Game/Blueprints/BP_Marine` (`GameplayStatics.GetPlayerCharacter` 0)))
  (set `self.As BP Marine` _asbp_marine)
  (set `self.CurrentHealth` (`self.Health`))
  (`|PlayMontage` (`self.Mesh`) "/Game/Characters/Enemy_Great_Spider/Animations/AMN_Teleport.AMN_Teleport"
    (:`OnCompleted`
      (set `self.isGround` true)
      (`self.FollowPlayer`))))

(event `self.ReceiveAnyDamage`
  (params (Damage :type "Float (single-precision)") (DamageType :type "DamageType Object Reference") (InstigatedBy :type "Controller Object Reference") (DamageCauser :type "Actor Object Reference"))
  (if (`self.IsAlive`)
    (bind _death (`self.TakeDamage` Damage))
    (`GameplayStatics.SpawnSoundAtLocation` "/Game/Sounds/FoleyFlesh/Stereo/FoleyImpact_cue.FoleyImpact_cue" (`self.K2_GetActorLocation`) (struct) 1.0 1.0 0.0 null null)
    (bind _output_get (set `self.IsAlive` (not _death)))
    (if _output_get
      _)))

(event `self.AttackRadius.OnComponentBeginOverlap`
  (params (OverlappedComponent :type "PrimitiveComponent Object Reference") (OtherActor :type "Actor Object Reference") (OtherComp :type "PrimitiveComponent Object Reference") (OtherBodyIndex :type Integer) (bFromSweep :type Boolean) (SweepResult :type "HitResult Structure (by ref)"))
  (cast `/Game/Blueprints/BP_Marine` OtherActor)
  (set `self.attackRange` true)
  (`self.Attack`))

(event `self.AttackRadius.OnComponentEndOverlap`
  (params (OverlappedComponent :type "PrimitiveComponent Object Reference") (OtherActor :type "Actor Object Reference") (OtherComp :type "PrimitiveComponent Object Reference") (OtherBodyIndex :type Integer))
  (cast `/Game/Blueprints/BP_Marine` OtherActor)
  (set `self.attackRange` false))

(event `self.ReceiveTick`
  (params (DeltaSeconds :type "Float (single-precision)"))
  (`/Engine/EditorBlueprintResources/StandardMacros.DoOnce` false :!label _label
    (:`Completed`
      (`self.FollowPlayer`
        (:`OnSucces`
          (goto _label :!via `Reset`))
        (:`On Fail`
          (goto _label :!via `Reset`))))))

(event `Attack`
  (bind _charactermovement (`self.CharacterMovement`))
  (if (and (`self.isGround`) (`self.IsAlive`) (`/Game/Blueprints/BP_Marine.playerIsAlive` (`self.As BP Marine`))) :!label _label_2
    (if (and (`self.attackRange`) (not (`self.IsAttacking`)))
      (`|PlayMontage` (`self.Mesh`) "/Game/Characters/Enemy_Great_Spider/Animations/AMN_Spider.AMN_Spider"
        (:`then`
          _)
        (:`OnCompleted`
          (if (`self.IsAlive`)
            (`ActorComponent.Activate` _charactermovement false)
            (goto _label_2)
            (else
              _))))
      (`ActorComponent.Deactivate` _charactermovement))))

(fn `ChangeMaterial`
  (params (MaterialIndex :type Integer))
  (`PrimitiveComponent.SetMaterial` (`self.Mesh`) 0 (`|GetArrayItem` (`self.EnemyMaterials`) MaterialIndex)))

(fn `ChangeMaterialSystemBuff`
  (params (Value :type "Float (double-precision)"))
  (locals (healtLocabuff :type Boolean :default false) (damagelocalbuff :type Boolean :default false))
  ; HealthUpgradeAviable
  (bind _output_get (set `local.healtLocabuff` (`self.UpgradeAviable`)))
  (`KismetSystemLibrary.PrintString` (`KismetStringLibrary.Conv_BoolToString` _output_get))
  (if _output_get
    (`self.HealthUpgrade` Value)
    (`self.ChangeMaterial` 1)
    (`KismetSystemLibrary.PrintString` "HealthBuff"))
  ; Damage Upgrade Aviable
  (bind _output_get_2 (set `local.damagelocalbuff` (`self.UpgradeAviable`)))
  (`KismetSystemLibrary.PrintString` (`KismetStringLibrary.Conv_BoolToString` _output_get_2))
  (if _output_get_2
    (`self.DamageUpgrade` Value)
    (`self.ChangeMaterial` 0)
    (`KismetSystemLibrary.PrintString` "DamageBuff")
    ; AllDebuffAviable
    (if (and (`local.healtLocabuff`) (`local.damagelocalbuff`))
      (`self.ChangeMaterial` 2)
      (`KismetSystemLibrary.PrintString` "AllByff")))
  (return))

(fn `DamagePlayer`
  (`GameplayStatics.ApplyDamage` (`GameplayStatics.GetPlayerCharacter` 0) (`self.DamageValue`))
  (return))

(fn `DamageUpgrade`
  (params (UpgradeValue :type "Float (double-precision)"))
  (set `self.DamageValue` (* (`self.DamageValue`) UpgradeValue)))

(fn `DropAviable`
  (returns (ReturnValue :type Boolean))
  (return (>= (`/Game/Blueprints/BP_Marine.DropChance` (`self.As BP Marine`)) (`KismetMathLibrary.RandomFloatInRange` 0.0 100.0))))

(fn `DropSystem`
  ; HealthDrop
  (if (`self.DropAviable`)
    (`|SpawnActorFromClass` "/Game/Blueprints/BP_PickHealth.BP_PickHealth_C" (`KismetMathLibrary.MakeTransform` (+ (`self.K2_GetActorLocation`) (`KismetMathLibrary.MakeVector` (`KismetMathLibrary.RandomFloatInRange` -30.0 30.0) (`KismetMathLibrary.RandomFloatInRange` -30.0 30.0)))) "Undefined" "MultiplyWithRoot" null null))
  ; RiffleDrop
  (if (`self.DropAviable`)
    (`|SpawnActorFromClass` "/Game/Blueprints/BP_RiffleBuff.BP_RiffleBuff_C" (`KismetMathLibrary.MakeTransform` (+ (`self.K2_GetActorLocation`) (`KismetMathLibrary.MakeVector` (`KismetMathLibrary.RandomFloatInRange` -30.0 30.0) (`KismetMathLibrary.RandomFloatInRange` -30.0 30.0)))) "Undefined" "MultiplyWithRoot" null null)))

(fn `HealthUpgrade`
  (params (`UpgradeValuıe` :type "Float (double-precision)"))
  (bind _output_get (set `self.Health` (* (`self.Health`) `UpgradeValuıe`)))
  (set `self.CurrentHealth` _output_get))

(fn `IsAttacking`
  (returns (isPlay :type Boolean))
  (return (`AnimInstance.Montage_IsPlaying` (`SkeletalMeshComponent.GetAnimInstance` (`self.Mesh`)) "/Game/Characters/Enemy_Great_Spider/Animations/AMN_Spider.AMN_Spider")))

(fn `IsAttackRange`
  (returns (IsRange :type Boolean))
  (return (>= 0.0 (`self.GetDistanceTo` (`GameplayStatics.GetPlayerCharacter` 0) self))))

(fn `TakeDamage`
  (params (Damage :type "Float (double-precision)"))
  (returns (death :type Boolean))
  (bind _output_get (set `self.CurrentHealth` (`KismetMathLibrary.FClamp` (- (`self.CurrentHealth`) Damage) 0.0 (`self.Health`))))
  (return (== _output_get 0.0)))

(fn `UpgradeAviable`
  (returns (Aviable :type Boolean))
  (return (> (`self.UpgradeChance`) (`KismetMathLibrary.RandomFloatInRange` 0.0 100.0))))

(fn `UserConstructionScript`)